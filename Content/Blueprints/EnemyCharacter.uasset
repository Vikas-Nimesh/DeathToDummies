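; Enemy character Blueprint that dies when its health runs out and supports a configurable body color.
; On receiving damage it runs the parent handler, then at zero or lower Health sets IsDead, detaches its controller and destroys itself after a short delay.
; The construction script creates a dynamic material instance on the mesh and applies BodyColor to it.
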(event `self.OnReceiveDamage`
  (`parent.OnReceiveDamage`)
  (if (<= (`self.Health`) 0)
    (set `self.isDead` true)
    (`self.DetachFromControllerPendingDestroy`)
    (`KismetSystemLibrary.Delay` 4.0)
    (`self.K2_DestroyActor`)))

(fn `UserConstructionScript`
  (bind _returnvalue (`PrimitiveComponent.CreateDynamicMaterialInstance` (`self.Mesh`) 0 null "None"))
  (bind _output_get (set `self.Dynamic Material` _returnvalue))
  (`MaterialInstanceDynamic.SetVectorParameterValue` _output_get "BodyColor" (`self.BodyColor`)))