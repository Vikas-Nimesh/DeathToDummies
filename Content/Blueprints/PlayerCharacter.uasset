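; Player character Blueprint that handles movement, mouse look and weapon firing.
; On BeginPlay it spawns a weapon actor and attaches it to the mesh's WeaponSocket.
; Fire press and release are forwarded to that weapon's StartFire and StopFire.
; Move axes follow the camera's forward and right vectors, while look axes feed controller pitch and yaw.
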(event `InputAction|Fire`
  (params (Key :type "Key Structure"))
  (bind _weapon (`self.Weapon`))
  (:`Pressed`
    (`/Game/Blueprints/WeaponBlueprint.StartFire` _weapon))
  (:`Released`
    (`/Game/Blueprints/WeaponBlueprint.StopFire` _weapon)))

(event `self.ReceiveBeginPlay`
  (bind _mesh (`self.Mesh`))
  (bind _returnvalue (`|SpawnActorFromClass` "/Game/Blueprints/WeaponBlueprint.WeaponBlueprint_C" (`SceneComponent.K2_GetComponentToWorld` _mesh) "Undefined" "OverrideRootScale" null null))
  (bind _output_get (set `self.Weapon` _returnvalue))
  (`self.K2_AttachToComponent` _output_get _mesh "WeaponSocket" "SnapToTarget" "SnapToTarget" "SnapToTarget" true))

(event `InputAxis|MoveUpDown`
  (params (AxisValue :type "Float (single-precision)"))
  ;[1 1 1] Keyboard Movement
  (`self.AddMovementInput` (`KismetMathLibrary.GetForwardVector` (`SceneComponent.K2_GetComponentRotation` (`self.Camera`))) AxisValue))

(event `InputAxis|MoveRightLeft`
  (params (AxisValue :type "Float (single-precision)"))
  ;[1 1 1] Keyboard Movement
  (`self.AddMovementInput` (`KismetMathLibrary.GetRightVector` (`SceneComponent.K2_GetComponentRotation` (`self.Camera`))) AxisValue))

(event `InputAxis|LookUpDown`
  (params (AxisValue :type "Float (single-precision)"))
  ;[1 1 1] Mouse Movement
  (`self.AddControllerPitchInput` AxisValue))

(event `InputAxis|LookRightLeft`
  (params (AxisValue :type "Float (single-precision)"))
  ;[1 1 1] Mouse Movement
  (`self.AddControllerYawInput` AxisValue))

(fn `UserConstructionScript`)