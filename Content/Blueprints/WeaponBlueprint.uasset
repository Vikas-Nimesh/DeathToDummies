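; Weapon Blueprint for an automatic hitscan gun that fires from StartFire until StopFire is called.
; StartFire spawns muzzle flash and gun sound once through a DoOnce, then re-triggers itself on a looping timer.
; Each shot line-traces forward from LaserBeam, damaging EnemyCharacter hits or spawning impact effects on other hits.
; StopFire clears the timer, stops the effects and resets the DoOnce; the cooldown logic is unconnected.
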(event `StartFire`
  (bind _laserbeam (`self.LaserBeam`))
  (bind _laserspawn (`self.LaserSpawn`))
  (bind _returnvalue (`SceneComponent.K2_GetComponentLocation` _laserbeam))
  (`|ExecutionSequence`
    (:`then_0`
      ;[1 1 1] Sound & FX
      (`/Engine/EditorBlueprintResources/StandardMacros.DoOnce` false :!label _label ; Play Muzzle FX and Animation Only Once
        (:`Completed`
          (`|ExecutionSequence`
            (:`then_0`
              (bind _returnvalue_2 (`GameplayStatics.SpawnEmitterAttached` "/Game/GunFX/ParticleSystems/Weapons/AssaultRifle/Muzzle/P_AssaultRifle_MF.P_AssaultRifle_MF" _laserspawn "None" (`SceneComponent.K2_GetComponentLocation` _laserspawn) (`SceneComponent.K2_GetComponentRotation` _laserspawn) (1.0 1.0 1.0) "KeepWorldPosition")))
            (:`then_1`
              (bind _returnvalue_3 (`GameplayStatics.SpawnSoundAttached` "/Game/Audio/GunSound.GunSound" _laserspawn "None" (0.0 0.0 0.0) (struct) "KeepRelativeOffset" true 2.0 1.0 0.0 null null false))
              (set `self.GunSound` _returnvalue_3))))))
    (:`then_1`
      ;[1 1 1] Bullets RayCasting
      (bind _outhit (`KismetSystemLibrary.LineTraceSingle` :`Start` _returnvalue :`End` (+ _returnvalue (* (`KismetMathLibrary.GetForwardVector` (`SceneComponent.K2_GetComponentRotation` _laserbeam)) (`KismetMathLibrary.Conv_DoubleToVector` (`self.Weapon Range`)))) :`TraceChannel` "TraceTypeQuery1" :`DrawDebugType` "ForOneFrame"))
      (bind (_bblockinghit _binitialoverlap _time _distance _location _impactpoint _normal _impactnormal _physmat _hitactor) (`GameplayStatics.BreakHitResult` _outhit))
      (bind _output_get (set `self.Hit Actor` _hitactor))
      (bind _asenemy_character (cast `/Game/Blueprints/EnemyCharacter` _output_get)
        (:`then`
          (`/Game/Blueprints/BaseCharacter.Receive Damage` _asenemy_character (`self.WeaponDamage`))
          (`GameplayStatics.SpawnEmitterAtLocation` "/Game/FX/EnemyImpact.EnemyImpact" (`self.K2_GetActorLocation` _asenemy_character)))
        (:`CastFailed`
          (`GameplayStatics.SpawnEmitterAtLocation` "/Game/GunFX/ParticleSystems/Weapons/AssaultRifle/Impacts/P_AssaultRifle_IH.P_AssaultRifle_IH" _impactpoint (`KismetMathLibrary.Conv_VectorToRotator` _impactnormal))
          (`KismetSystemLibrary.Delay` 0.5)
          (`GameplayStatics.SpawnSoundAtLocation` null _impactpoint (struct) 1.0 1.0 0.0 null null))))
    (:`then_2`
      (bind _returnvalue_4 (`KismetSystemLibrary.K2_SetTimer` null "StartFire" 0.05 true)))))

(event `StopFire`
  (`|ExecutionSequence`
    (:`then_0`
      (`KismetSystemLibrary.K2_ClearAndInvalidateTimerHandle` (stale `StartFire` _returnvalue_4)))
    (:`then_1`
      ;[1 1 1] Sound & FX
      (`ActorComponent.K2_DestroyComponent` (stale `StartFire` _returnvalue_2))
      (`AudioComponent.Stop` (`self.GunSound`)))
    (:`then_2`
      (goto _label :!via `Reset`))))

(fn `UserConstructionScript`)